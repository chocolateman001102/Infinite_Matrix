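; Projectile actor that flies along world X at a speed based on its shooter's forward speed.
; SetSpeed stores the shooter as Player and adds its ForwardSpeed to a base speed.
; Tick applies a swept world offset, destroying the actor only if a single frame's step reaches a large threshold, not on accumulated distance.
; The Bullet component also destroys the actor when an overlap ends, rather than begins.
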(event OnComponentEndOverlap(Bullet)
  (params (OverlappedComponent :type Primitive%20Component%20Object%20Reference) (OtherActor :type Actor%20Object%20Reference) (OtherComp :type Primitive%20Component%20Object%20Reference) (OtherBodyIndex :type Integer))
  (Actor|DestroyActor))

(event EventBeginPlay)

(event Collision|EventActorBeginOverlap
  (params (OtherActor :type Actor%20Object%20Reference)))

(event EventTick
  (params (DeltaSeconds :type Float%20%28single-precision%29))
  (bind _speed (Variables|Default|Getspeed))
  (bind _returnvalue (+ _speed 1.0))
  (bind _returnvalue_2 (* DeltaSeconds _returnvalue))
  (if (>= _returnvalue_2 5e+03)
    (Actor|DestroyActor)
    (else
      (Transformation|AddActorWorldOffset (Math|Vector|MakeVector _returnvalue_2 0.0 0.0) true))))

(fn ConstructionScript)

(fn SetSpeed
  (params (shooter :type BP%20Player%20Object%20Reference))
  (Variables|Default|SetPlayer shooter)
  (Variables|Default|Setspeed (+ 1e+03 (Variables|/Game/InfiniteMatrix/Blueprints/BP_Player.BP_Player_C|GetForwardSpeed%20 shooter))))